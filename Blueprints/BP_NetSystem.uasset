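; Python-driven actor that generates a synthetic pose dataset of Zenit-2 rocket debris seen from a chaser camera.
; Each comma-separated Python message supplies a pose and time step, spawning debris with remapped axes and positioning a net mesh by step.
; A timed event captures the render target to PNG, logs pose to CSV and saves camera intrinsics.
; It returns the filename to Python, then resets the net's transform and destroys the debris.
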(event Custom|Update%20Rotation
  (bind _chasercamera (Variables|Default|GetChaserCamera))
  (bind _python_communication (Variables|Default|GetPython%20Communication))
  (Transformation|SetActorRotation (stale Custom|On%20Python%20Reply _output_get_9) (Math|Rotator|MakeRotator (stale Custom|On%20Python%20Reply _output_get_7) (stale Custom|On%20Python%20Reply _output_get_5) (stale Custom|On%20Python%20Reply _output_get_6)))
  (Development|PrintString (Utilities|String|Append "Updated rotation aftet tick" (Utilities|String|ToString(Rotator) (Transformation|GetActorRotation (stale Custom|On%20Python%20Reply _output_get_9)))) true true "(R=1.000000,G=0.316616,B=0.913796,A=1.000000)" 1e+02)
  (Development|PrintString (Utilities|String|ToString(Transform) (Transformation|GetRelativeTransform (Variables|/Script/Engine.Actor|GetRootComponent (stale Custom|On%20Python%20Reply _output_get_9)))) true true "(R=0.467671,G=1.000000,B=0.215493,A=1.000000)" 2e+01)
  (Rendering|SceneCapture|CaptureScene (Variables|Default|GetSceneCaptureComponent2D) :!class /Script/Engine.SceneCaptureComponent2D)
  (bind _result (Math|Integer|IncrementInt (Variables|Default|GetFileCounter))
    (:%20%20
      (bind _output_get (Variables|Default|SetFileName (Utilities|String|Append (Utilities|String|ToString(Text) (Utilities|Text|FormatText "{FileImg}_{FileCounter}" (Variables|Default|GetFileImg) _result)) ".png")))
      (bind _output_get_2 (Variables|Default|SetFilePath "C:/Users/hahaha/Desktop/shubhrik/UrsoNet-master/datasets/Datasets_UE_satellite/"))
      (Rendering|ExportRenderTarget "/Game/Render_Cam1/NewTextureRenderTarget2D.NewTextureRenderTarget2D" _output_get_2 _output_get)
      (if (Class|BlueprintPathsLibrary|FileExists (Utilities|String|Append "" _output_get_2 _output_get))
        (bind _returnvalue (Actor|GetActorOfClass "/Game/Blueprints/BPA_Zenit-2Rocket.BPA_Zenit-2Rocket_C"))
        (bind _output_get_3 (Variables|Default|SetOut_Data _output_get))
        (bind _imagefilesfilename (Class|FileWriter|AppendPosetoCSV "/Script/Satellite_tether.Default__FileWriter" (/ (Math|Vector|MakeVector (.Y (Math|Vector|BreakVector (.Location (Math|Transform|BreakTransform (Transformation|GetActorTransform (stale Custom|On%20Python%20Reply _returnvalue_2)))))) (.Z (Math|Vector|BreakVector (.Location (Math|Transform|BreakTransform (Transformation|GetActorTransform (stale Custom|On%20Python%20Reply _returnvalue_2)))))) (.X (Math|Vector|BreakVector (.Location (Math|Transform|BreakTransform (Transformation|GetActorTransform (stale Custom|On%20Python%20Reply _returnvalue_2))))))) "100.000000,100.000000,100.000000") (Math|Rotator|MakeRotator (.Pitch (Math|Rotator|BreakRotator (Transformation|GetActorRotation _returnvalue))) (.Yaw (Math|Rotator|BreakRotator (Transformation|GetActorRotation _returnvalue))) (.Roll (Math|Rotator|BreakRotator (Transformation|GetActorRotation _returnvalue)))) _output_get (stale Custom|On%20Python%20Reply _output_get_8)))
        (Default|SendDatatoPyScript (Variables|Default|GetPython%20Communication) _output_get_3)
        (Development|PrintString _imagefilesfilename true true "(R=0.945679,G=1.000000,B=0.128853,A=1.000000)" 3e+01)
        (bind _desiredview (Class|CameraComponent|GetCameraView _chasercamera 1e+01))
        (Development|PrintString (Utilities|String|ToString(Integer) (.ViewMatrix (Class|GameplayStatics|GetViewProjectionMatrix _desiredview))))
        (Development|PrintString (Utilities|String|ToString(Integer) (.ProjectionMatrix (Class|GameplayStatics|GetViewProjectionMatrix _desiredview))))
        (Class|FileWriter|SaveCameraInstrinsicMatrix "/Script/Satellite_tether.Default__FileWriter" (Variables|/Script/Engine.CameraComponent|GetFieldOfView _chasercamera) 1.92e+03 1.08e+03 "/Saved Data/")
        (Transformation|SetRelativeTransform (Variables|Actor|GetNetMesh) (Math|Transform|MakeTransform "0, 0, 0" "0, 0, 0" "0.000000,0.000000,0.000000") false false)
        (Actor|DestroyActor (stale Custom|On%20Python%20Reply _output_get_9))
        (Utilities|IsValid (Variables|Default|GetDebris)
          (:Is%20Valid
            (Development|PrintString "Debris not destroyed"))
          (:Is%20Not%20Valid
            (if (Default|CheckPythonConnected _python_communication)
              (EventDispatchers|BindEventtoIncomingDatafromPython _python_communication (delegate Custom|On%20Python%20Reply)))))
        (else
          (Development|PrintString (Utilities|String|Append (Utilities|String|Append "" _output_get_2 _output_get) " does not exist")))))))

(event Custom|On%20Python%20Reply
  (params (Data :type String))
  (bind _netmesh (Variables|Actor|GetNetMesh))
  (bind _chasercamera (Variables|Default|GetChaserCamera))
  (bind _returnvalue (Transformation|GetWorldLocation _chasercamera))
  (bind (_x _y _z) (Class|KismetMathLibrary|BreakVector3f _returnvalue))
  (bind _output_get (Variables|Default|SetData Data))
  (for (_array_element _array_index) (Utilities|String|ParseIntoArray _output_get ",")
    (if (== _array_index 0)
      (bind _output_get_2 (Variables|Default|Setx (Math|Conversions|ToFloat(Integer) _array_element))))
    (if (== _array_index 1)
      (bind _output_get_3 (Variables|Default|Sety (Math|Conversions|ToFloat(Integer) _array_element))))
    (if (== _array_index 2)
      (bind _output_get_4 (Variables|Default|Setz (Math|Conversions|ToFloat(Integer) _array_element))))
    (if (== _array_index 3)
      (bind _output_get_5 (Variables|Default|Setroll (Math|Conversions|ToFloat(Integer) _array_element))))
    (if (== _array_index 4)
      (bind _output_get_6 (Variables|Default|Setpitch (Math|Conversions|ToFloat(Integer) _array_element))))
    (if (== _array_index 5)
      (bind _output_get_7 (Variables|Default|Setyaw (Math|Conversions|ToFloat(Integer) _array_element))))
    (if (== _array_index 6)
      (bind _output_get_8 (Variables|Default|Sett (Math|Float|Truncate (Math|Conversions|ToFloat(Integer) _array_element))))
      (switch int _output_get_8
        (:0
          (Transformation|AddWorldOffset _netmesh "0, 0, 0" false false)
          (Transformation|SetWorldScale3D _netmesh "0, 0, 0"))
        (:5
          (Transformation|AddWorldOffset _netmesh "700.000000,0.000000,0.000000" true false)
          (Transformation|SetWorldScale3D _netmesh "0.200000,0.200000,0.200000"))
        (:10
          (Transformation|AddWorldOffset _netmesh "1500.000000,0.000000,0.000000" true false)
          (Transformation|SetWorldScale3D _netmesh "0.300000,0.300000,0.300000"))
        (:15
          (Transformation|AddWorldOffset _netmesh "2000.000000,0.000000,0.000000" true false)
          (Transformation|SetWorldScale3D _netmesh "0.550000,0.550000,0.550000")))
      (Development|PrintString (Utilities|String|Append "Chaser Camera position and orientation" (Utilities|String|ToString(Transform) (Transformation|GetWorldTransform _chasercamera))))
      (Development|PrintString (Utilities|String|Append "Position of target in world" (Utilities|String|ToString(Vector) (Math|Vector|MakeVector (* (+ _x _output_get_4) 1e+02) (* (+ _y _output_get_2) 1e+02) (* (+ _z _output_get_3) 1e+02)))) true true "(R=0.864023,G=1.000000,B=0.708147,A=1.000000)" 1e+02)
      (Utilities|IsValid (Variables|Default|GetDebris)
        (:Is%20Valid
          (Actor|DestroyActor (Variables|Default|GetDebris)))
        (:Is%20Not%20Valid
          _))
      (bind _returnvalue_2 (Game|SpawnActorfromClass "/Game/Blueprints/BPA_Zenit-2Rocket.BPA_Zenit-2Rocket_C" (Math|Transform|MakeTransform (Math|Vector|MakeVector (* (+ _x _output_get_4) 1e+02) (* (+ _y _output_get_2) 1e+02) (* (+ _z _output_get_3) 1e+02)) (Math|Rotator|MakeRotator _output_get_7 _output_get_5 _output_get_6) "0.050000,0.050000,0.050000") "Undefined" "OverrideRootScale" 0 0))
      (bind _output_get_9 (Variables|Default|SetDebris _returnvalue_2))
      (Utilities|Time|SetTimerbyEvent (delegate Custom|Update%20Rotation) (stale EventTick DeltaSeconds)))))

(event EventBeginPlay
  (bind _returnvalue (Actor|GetActorOfClass "/PyRuntimeUtility/BP_Python_Runtime_Connection.BP_Python_Runtime_Connection_C"))
  (bind _output_get (Variables|Default|SetPython%20Communication _returnvalue))
  (EventDispatchers|BindEventtoIncomingDatafromPython _output_get (delegate Custom|On%20Python%20Reply))
  (Default|StartPythonConnection _output_get))

(event EventTick
  (params (DeltaSeconds :type Float%20%28single-precision%29)))

(fn ConstructionScript)

(fn OnRepDebris)